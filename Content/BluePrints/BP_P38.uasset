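; Player-controlled P-38 plane pawn that constantly flies forward, steers in pitch and roll, and fires rockets.
; Tick feeds forward movement input, while the Enhanced Input IA_PitchRoll action applies frame-rate-scaled local rotation.
; IA_Fire spawns BP_Rocket at the Arrow component with the plane as owner and instigator.
; Propeller-spin helpers, older axis-based steering and dynamic-material setup remain, but none are wired into running logic.
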(event `InputAxis|Pitch`
  (params (AxisValue :type "Float (single-precision)"))
  ;[1 1 1] Pitch
)

(event `InputAxis|Roll`
  (params (AxisValue :type "Float (single-precision)"))
  ;[1 1 1] Roll
)

(event `EnhancedInput|/Game/BluePrints/Input/IA_Pitch`
  (params (ActionValue :type "Float (double-precision)") (ElapsedSeconds :type "Float (double-precision)") (TriggeredSeconds :type "Float (double-precision)") (InputAction :type "InputAction Object Reference" :default "/Game/BluePrints/Input/IA_Pitch.IA_Pitch"))
  ;[1 1 1] InputAction IA_Pitch
)

(event `EnhancedInput|/Game/BluePrints/Input/IA_Roll`
  (params (ActionValue :type "Float (double-precision)") (ElapsedSeconds :type "Float (double-precision)") (TriggeredSeconds :type "Float (double-precision)") (InputAction :type "InputAction Object Reference" :default "/Game/BluePrints/Input/IA_Roll.IA_Roll"))
  ;[1 1 1] InputAction IA_Roll
)

(event `self.ReceiveTick`
  (params (DeltaSeconds :type "Float (single-precision)"))
  ;[1 1 1] 앞으로 이동
  (`|ExecutionSequence`
    (:`then_0`
      (`self.AddMovementInput` (`self.GetActorForwardVector`)))))

(event `EnhancedInput|/Game/BluePrints/Input/IA_PitchRoll`
  (params (ActionValue :type "Vector2D Structure") (ElapsedSeconds :type "Float (double-precision)") (TriggeredSeconds :type "Float (double-precision)") (InputAction :type "InputAction Object Reference" :default "/Game/BluePrints/Input/IA_PitchRoll.IA_PitchRoll"))
  ;[1 1 1] InputAction IA_PitchRoll
  (:`Triggered`
    (`self.K2_AddActorLocalRotation` (* (`KismetMathLibrary.MakeRotator` ActionValue_X ActionValue_Y) (* (`GameplayStatics.GetWorldDeltaSeconds`) (`self.Rotate_Speed`))))))

(event `EnhancedInput|/Game/BluePrints/Input/IA_Fire`
  (params (ActionValue :type Boolean) (ElapsedSeconds :type "Float (double-precision)") (TriggeredSeconds :type "Float (double-precision)") (InputAction :type "InputAction Object Reference" :default "/Game/BluePrints/Input/IA_Fire.IA_Fire"))
  ;[1 1 1] Fire
  (:`Triggered`
    (`|SpawnActorFromClass` "/Game/BluePrints/BP_Rocket.BP_Rocket_C" (`SceneComponent.K2_GetComponentToWorld` (`self.Arrow`)) "Undefined" "OverrideRootScale" self self)))

(event `RotateProreller`
  (params (Where :type "StaticMeshComponent Object Reference"))
  ;[1 1 1] 커스텀 이벤트로 프로펠러 회전
  (`SceneComponent.K2_AddLocalRotation` Where (`KismetMathLibrary.MakeRotator` (* (`GameplayStatics.GetWorldDeltaSeconds`) 5000.0)) false false))

(fn `Rotate_Propeller`
  (params (Where :type "StaticMeshComponent Object Reference"))
  ;[1 1 1] 프로펠러 회전
  (`SceneComponent.K2_AddRelativeRotation` Where (`KismetMathLibrary.MakeRotator` (* (`GameplayStatics.GetWorldDeltaSeconds`) (`self.Propeller_Rotate_Speed`))) false false))

(fn `UserConstructionScript`)